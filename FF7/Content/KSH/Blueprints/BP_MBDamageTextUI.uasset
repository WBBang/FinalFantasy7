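; BP_MBDamageTextUI is a world-space text actor, named for damage text, that animates once when spawned and then destroys itself.
; On BeginPlay it caches its start location and plays the DamageText timeline.
; A single vector track drives the TextRender: Z offsets it vertically from the start, while Y sets only its X scale, as the Y-scale call is disconnected.
; The Blueprint does not set the text itself.
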(event `self.ReceiveBeginPlay`
  (set `self.StartPos` (`self.K2_GetActorLocation`))
  (bind (_direction _newtrack_0) (`Timeline|DamageText`)
    (:`Update`
      (`SceneComponent.K2_SetWorldLocation` (`self.textRender`) (+ (`KismetMathLibrary.MakeVector` 0.0 0.0 (.z _newtrack_0)) (`self.StartPos`)) false false)
      (`TextRenderComponent.SetXScale` (`self.textRender`) (.y _newtrack_0)))
    (:`Finished`
      (`self.K2_DestroyActor`))))

(fn `UserConstructionScript`)