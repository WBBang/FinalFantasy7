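; Test character Blueprint for Barrett, driven by direct keyboard events.
; Shift toggles sprint speed while held, WASD only sets flags, and Space is a roll stub, blocked when sprinting with a direction held, that sets location to the origin and plays an unassigned montage.
; Key 1 damages the MiddleBossCharacter for testing.
; Sphere-trace camera lock-on and attack/aim montages exist but are disconnected.
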(event `Key|One`
  (params (Key :type "Key Structure"))
  (:`Pressed`
    (bind _returnvalue (`GameplayStatics.GetActorOfClass` "/Script/FF7.MiddleBossCharacter"))
    (`MiddleBossCharacter.MiddleBossDamaged` _returnvalue 1.0)))

(event `Key|Two`
  (params (Key :type "Key Structure")))

(event `Key|Tab` :overrideparent false
  (params (Key :type "Key Structure"))
  ;[1 0.3519 0] Tap Key 를 눌렀을 때 Camera 락온
)

(event `Key|Tab` :overrideparent false
  (params (Key :type "Key Structure")))

(event `Key|LeftShift` :overrideparent false
  (params (Key :type "Key Structure"))
  ;[1 1 1] Sprint
  (:`Pressed`
    (set `CharacterMovementComponent.MaxWalkSpeed` 1000.0 (`self.CharacterMovement`))
    (set `self.LeftShift` true))
  (:`Released`
    (set `CharacterMovementComponent.MaxWalkSpeed` 400.0 (`self.CharacterMovement`))
    (set `self.LeftShift` false)))

(event `Key|W` :overrideparent false
  (params (Key :type "Key Structure"))
  ;[1 1 1] 이동
  ;;[1 0 0] 앞
  (:`Pressed`
    (set `self.W` true))
  (:`Released`
    (set `self.W` false)))

(event `Key|LeftMouseButton` :overrideparent false
  (params (Key :type "Key Structure")))

(event `Key|A` :overrideparent false
  (params (Key :type "Key Structure"))
  ;[1 1 1] 이동
  ;;[0 1 0] 왼쪽
  (:`Pressed`
    (set `self.A` true))
  (:`Released`
    (set `self.A` false)))

(event `Key|S` :overrideparent false
  (params (Key :type "Key Structure"))
  ;[1 1 1] 이동
  ;;[0 0 1] 뒤
  (:`Pressed`
    (set `self.S` true))
  (:`Released`
    (set `self.S` false)))

(event `Key|D` :overrideparent false
  (params (Key :type "Key Structure"))
  ;[1 1 1] 이동
  ;;[1 1 0] 오른쪽
  (:`Pressed`
    (set `self.D` true))
  (:`Released`
    (set `self.D` false)))

(event `Key|SpaceBar` :overrideparent false
  (params (Key :type "Key Structure"))
  ;[1 1 1] 구르기(Sprint 중에는 안됨)
  (:`Pressed`
    (set `self.SpaceBar` true)
    (if (and (`self.SpaceBar`) (`KismetMathLibrary.BooleanNAND` (`self.LeftShift`) (or (`self.W`) (`self.A`) (`self.S`) (`self.D`))))
      (`self.K2_SetActorLocation` (0.0 0.0 0.0))
      (`|PlayMontage` (`self.Mesh`))))
  (:`Released`
    (set `self.SpaceBar` false)))

(event `self.ReceiveTick`
  (params (DeltaSeconds :type "Float (single-precision)")))

(fn `UserConstructionScript`)